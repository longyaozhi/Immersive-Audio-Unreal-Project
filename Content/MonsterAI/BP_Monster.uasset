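; BP_Monster is an AI monster pawn that chases the player and catches them on contact.
; Every tick it issues AIMoveTo toward the player's current location.
; A collision overlap with BP_FirstPersonCharacter calls that character's WhenCaught.
; BeginPlay registers the monster in a collection and sets a footsteps timer, whose event checks velocity before a FlipFlop with no visible outputs.
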(event OnComponentBeginOverlap(Collision)
  (params (OverlappedComponent :type Primitive%20Component%20Object%20Reference) (OtherActor :type Actor%20Object%20Reference) (OtherComp :type Primitive%20Component%20Object%20Reference) (OtherBodyIndex :type Integer) (bFromSweep :type Boolean) (SweepResult :type Hit%20Result%20Structure%20%28by%20ref%29))
  (bind _asbp_first_person_character (Utilities|Casting|CastToBP_FirstPersonCharacter OtherActor))
  (Default|WhenCaught _asbp_first_person_character))

(event Custom|footsteps
  (if (> (Math|Vector|VectorLength (Pawn|Components|CharacterMovement|GetLastUpdateVelocity (Variables|Character|GetCharacterMovement))) 0.0)
    (Utilities|FlowControl|FlipFlop)))

(event EventBeginPlay
  (Utilities|Set|Add 0 self)
  (Utilities|Time|SetTimerbyEvent (delegate Custom|footsteps) 0.75))

(event EventTick
  (params (DeltaSeconds :type Float%20%28single-precision%29))
  (AI|AIMoveTo (Variables|Character|GetCharacterMovement) self (Transformation|GetActorLocation (Game|GetPlayerCharacter 0)) 0 5.0 false))

(fn ConstructionScript)